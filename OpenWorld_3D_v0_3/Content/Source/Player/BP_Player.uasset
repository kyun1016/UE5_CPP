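; Player character Blueprint with an aimed magic stance, spell attack, crosshair HUD and debug keys for noise, damaging all enemies and random targeting.
; Zoom input switches stance, changing rotation mode, walk speed, crosshair and camera boom offset.
; Attacking in magic stance plays a montage whose notify camera-traces the aim point and fires through BPCAttacks from the hand socket.
; BPC_DamageSystem handles health and attack tokens, driving hit reactions and ragdoll death.
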(event OnDeath(BPC_DamageSystem)
  (bind _mesh (Variables|Character|GetMesh))
  ;[1 1 1] Dead
  (Physics|SetSimulatePhysics _mesh true)
  (Collision|SetCollisionEnabled _mesh "QueryAndPhysics")
  (Input|DisableInput (Game|GetPlayerController 0)))

(event OnDamageResponse(BPC_DamageSystem)
  (params (DamageResponse :type E_DamageResponse%20Enum :default "NewEnumerator0") (DamageCauser :type Actor%20Object%20Reference))
  (bind _returnvalue (Game|GetPlayerController 0))
  ;[1 1 1] Hit
  (Input|DisableInput _returnvalue)
  (Animation|Montage|PlayMontage (Variables|Character|GetMesh) "/Game/Source/Enemy/Animation/Sword/Montage_Sword_Hit.Montage_Sword_Hit"
    (:OnCompleted
      _)
    (:OnInterrupted
      _))
  (Input|EnableInput _returnvalue))

(event Custom|EnterMagicStance
  (bind _charactermovement (Variables|Character|GetCharacterMovement))
  ;[1 1 1] Change Stance
  (Variables|Default|SetStance "NewEnumerator1")
  (Variables|/Script/Engine.CharacterMovementComponent|SetbOrientRotationToMovement _charactermovement false)
  (Variables|/Script/Engine.CharacterMovementComponent|SetbUseControllerDesiredRotation _charactermovement true)
  (Variables|/Script/Engine.CharacterMovementComponent|SetMaxWalkSpeed _charactermovement (Variables|Default|GetMagicWalkSpeed))
  (Default|ShowCrosshair (Variables|Default|GetWB_CrosshairRef))
  (bind _aimalpha (Timeline|AimTimeline PlayFromStart)
    (:Update
      (Variables|/Script/Engine.SpringArmComponent|SetSocketOffset (Variables|Default|GetCameraBoom) (Math|Vector|Lerp(Vector) (Variables|Default|GetDefaultBoomOffset) (Variables|Default|GetAimBoomOffset) _aimalpha)))))

(event Custom|EnterDefaultStance
  (bind _charactermovement (Variables|Character|GetCharacterMovement))
  ;[1 1 1] Change Stance
  (Variables|Default|SetStance "NewEnumerator0")
  (Variables|/Script/Engine.CharacterMovementComponent|SetbOrientRotationToMovement _charactermovement true)
  (Variables|/Script/Engine.CharacterMovementComponent|SetbUseControllerDesiredRotation _charactermovement false)
  (Variables|/Script/Engine.CharacterMovementComponent|SetMaxWalkSpeed _charactermovement (Variables|Default|GetDefaultWalkSpeed))
  (Default|HideCrosshair (Variables|Default|GetWB_CrosshairRef))
  (Variables|/Script/Engine.SpringArmComponent|SetSocketOffset (Variables|Default|GetCameraBoom) (Variables|Default|GetDefaultBoomOffset))
  (Utilities|String|Reverse (Variables|Default|GetAimTimeline)))

(event Custom|DisplayHUD
  ;[1 1 1] HUD Crosshair
  (bind _wb_crosshairref (Variables|Default|GetWB_CrosshairRef)
    (:then
      (Widget|SetVisibility _wb_crosshairref "Visible"))
    (:else
      (bind _returnvalue (UserInterface|CreateWidget "/Game/Source/HUD/WB_Crosshair.WB_Crosshair_C"))
      (bind _output_get (Variables|Default|SetWB_CrosshairRef _returnvalue))
      (UserInterface|Viewport|AddtoViewport _output_get 0))))

(event Custom|DamageEnemy
  (params (OtherActor :type Actor%20Object%20Reference) (Hit :type Hit%20Result%20Structure))
  ;[1 1 1] Attack With Projectiles
  (Class|BPIDamagable|TakeDamage(Message) OtherActor (Variables|Default|GetDamageInfoMagic)))

(event Custom|ShootMagicSpell
  (bind _followcamera (Variables|Default|GetFollowCamera))
  (bind _mesh (Variables|Character|GetMesh))
  (bind _returnvalue (Transformation|GetSocketLocation _mesh "RightHandMiddle1"))
  (bind _returnvalue_2 (Transformation|GetWorldLocation _followcamera))
  (bind _returnvalue_3 (+ _returnvalue "-5.000000,-5.000000,5.000000"))
  ;[1 1 1] Magic Spell
  (if (Utilities|Enum|Equal(Enum) (Variables|Default|GetStance) "NewEnumerator1")
    (Variables|Default|SetbAnimAttack true)
    (Variables|Default|SetbCanMove false)
    (bind _notifyname (Animation|Montage|PlayMontage (Variables|Character|GetMesh) "/Game/Source/Player/Animation/Montage_Magic_Attack.Montage_Magic_Attack")
      (:OnCompleted
        (Variables|Default|SetbAnimAttack false :!label _label)
        (Variables|Default|SetbCanMove true)
        (Variables|Default|SetAttacking false))
      (:OnInterrupted
        (goto _label))
      (:OnNotifyBegin
        (switch name _notifyname
          (:Fire
            (Variables|Default|SetAttacking true)
            (bind (_outhit _returnvalue_4) (Collision|LineTraceByChannel _returnvalue_2 (+ _returnvalue_2 (* (Math|Vector|GetForwardVector _followcamera) 1e+04)) "TraceTypeQuery1" false 0 "None"))
            (Default|MagicSpell (Variables|Default|GetBPC_Attacks) (Math|Transform|MakeTransform _returnvalue_3 (Math|Rotator|FindLookatRotation _returnvalue_3 (Math|Vector|SelectVector (.Location (Collision|BreakHitResult _outhit)) (.TraceEnd (Collision|BreakHitResult _outhit)) _returnvalue_4)) "1.000000,1.000000,1.000000") (Variables|Default|GetTarget) (Variables|Default|GetDamageInfoMagic))))))))

(event Input|EnhancedActionEvents|EnhancedInputActionIA_Zoom
  (params (ActionValue :type Boolean) (ElapsedSeconds :type Float%20%28double-precision%29) (TriggeredSeconds :type Float%20%28double-precision%29) (InputAction :type Input%20Action%20Object%20Reference :default "/Game/Source/Input/Actions/IA_Zoom.IA_Zoom"))
  ;[1 1 1] Change Stance
  (:Started
    (CallFunction|EnterMagicStance))
  (:Completed
    (CallFunction|EnterDefaultStance)))

(event Input|EnhancedActionEvents|EnhancedInputActionIA_Attack
  (params (ActionValue :type Boolean) (ElapsedSeconds :type Float%20%28double-precision%29) (TriggeredSeconds :type Float%20%28double-precision%29) (InputAction :type Input%20Action%20Object%20Reference :default "/Game/Source/Input/Actions/IA_Attack.IA_Attack"))
  ;[1 1 1] Attack
  (if (not (Variables|Default|GetbAnimAttack))
    (CallFunction|ShootMagicSpell)))

(event EventBeginPlay
  (|CallParentFunction)
  (CallFunction|DisplayHUD))

(event Input|KeyboardEvents|3
  (params (Key :type Key%20Structure))
  (bind _returnvalue (Transformation|GetActorLocation))
  ;[0.0356 0.0356 0.0356] Debug - Enemy Patrol / Attack Toggle
  (:Pressed
    (Class|Actor|MakeNoise 1.0 self _returnvalue 0.0 "None")
    (Effects|SpawnEmitteratLocation "/Game/StarterContent/Particles/P_Explosion.P_Explosion" _returnvalue)
    (Audio|PlaySoundatLocation "/Game/StarterContent/Audio/Explosion_Cue.Explosion_Cue" _returnvalue "0, 0, 0" 1.0 1.0 0.0 0 0 0 0)))

(event Input|KeyboardEvents|X
  (params (Key :type Key%20Structure))
  ;[1 1 1] Damage System
  (:Pressed
    (bind _outactors (Actor|GetAllActorsOfClass "/Game/Source/Enemy/BP_Enemy_Base.BP_Enemy_Base_C"))
    (for _array_element _outactors
      (Default|TakeDamage _array_element (Variables|Default|GetDamageInfoMagic)))))

(event Input|KeyboardEvents|F
  (params (Key :type Key%20Structure))
  ;[1 1 1] Zoom
  (:Pressed
    (bind _outactors (Actor|GetAllActorsOfClass "/Script/OpenWorld_3D_v0_3.EnemyBase"))
    (Variables|Default|SetTarget (Utilities|Array|Get(acopy) _outactors (Math|Random|RandomInteger (Utilities|Array|Length _outactors))))
    (Development|PrintString (Utilities|String|ToString(Integer) (Math|Random|RandomInteger (Utilities|Array|Length _outactors)))))
  (:Released
    (Variables|Default|SetTarget 0)))

(fn ConstructionScript)

(fn GetCurrentHealth
  (return (Variables|/Game/Source/DamageSystem/BPC_DamageSystem.BPC_DamageSystem_C|GetHealth (Variables|Default|GetBPC_DamageSystem))))

(fn GetMaxHealth
  (return (Variables|/Game/Source/DamageSystem/BPC_DamageSystem.BPC_DamageSystem_C|GetMaxHealth (Variables|Default|GetBPC_DamageSystem))))

(fn GetTeamNumber
  (return (Variables|Default|GetTeamNumber)))

(fn Heal
  (params (Amount :type Float%20%28double-precision%29))
  (bind _health (Default|Heal (Variables|Default|GetBPC_DamageSystem) Amount))
  (return _health))

(fn IsAttacking
  (return (Variables|Default|GetAttacking)))

(fn IsDead
  (return (Variables|/Game/Source/DamageSystem/BPC_DamageSystem.BPC_DamageSystem_C|GetIsDead (Variables|Default|GetBPC_DamageSystem))))

(fn ReserveAttackToken
  (params (Amout :type Integer))
  (bind _success (Default|ReserveAttackToken (Variables|Default|GetBPC_DamageSystem) Amout))
  (return _success))

(fn ReturnAttackToken
  (params (Amout :type Integer))
  (Default|ReturnAttackToken (Variables|Default|GetBPC_DamageSystem) Amout)
  (return))

(fn TakeDamage
  (params (DamageInfo :type S%20Damage%20Info%20Structure) (DamageCauser :type Actor%20Object%20Reference))
  (bind _wasdamaged (Default|TakeDamage (Variables|Default|GetBPC_DamageSystem) DamageInfo DamageCauser))
  (return _wasdamaged))