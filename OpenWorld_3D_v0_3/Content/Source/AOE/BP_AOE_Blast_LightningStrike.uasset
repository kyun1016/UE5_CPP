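; Lightning strike blast area-of-effect actor that adds a temporary Niagara effect on top of its parent's behavior.
; On BeginPlay it runs the parent logic, spawns a Niagara component at four times scale and binds to the OnActive event.
; When OnActive fires, it destroys that component, so the effect only shows until the blast becomes active.
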(event Custom|OnActive_Event
  (Components|DestroyComponent (stale EventBeginPlay _returnvalue)))

(event EventBeginPlay
  (|CallParentFunction)
  (bind _returnvalue (AddComponent|AddNiagaraComponent false (Math|Transform|MakeTransform "0, 0, 0" "0, 0, 0" "4.000000,4.000000,4.000000")))
  (EventDispatchers|BindEventtoOnActive (delegate Custom|OnActive_Event)))

(event Collision|EventActorBeginOverlap
  (params (OtherActor :type Actor%20Object%20Reference))
  (|CallParentFunction OtherActor) ; This node is disabled and will not be called.\nDrag off pins to build functionality.
)

(event EventTick
  (params (DeltaSeconds :type Float%20%28single-precision%29))
  (|CallParentFunction DeltaSeconds) ; This node is disabled and will not be called.\nDrag off pins to build functionality.
)

(fn ConstructionScript
  (|CallParentFunction))