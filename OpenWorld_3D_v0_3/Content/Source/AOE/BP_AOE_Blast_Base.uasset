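; Base Blueprint for blast area-of-effect actors, adding one-shot visual and audio feedback to the parent AOE behavior.
; Trigger calls the parent, then binds the blast effect to OnActive, which plays the sound and spawns an attached particle emitter.
; The sound also emits noise with the player pawn as instigator.
; The actor destroys itself when the particles finish, or after a short delay without sound if no effect is set.
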(event Custom|SystemFinished
  (params (PSystem :type Particle%20System%20Component%20Object%20Reference))
  ;[1 1 1] Effect
  (Actor|DestroyActor))

(event Custom|SpawnBlastEffect
  ;[1 1 1] Effect
  (bind _effect (Variables|Default|GetEffect)
    (:then
      (CallFunction|PlayBlastSound)
      (bind _returnvalue (Effects|SpawnEmitterAttached _effect (Variables|Default|GetDefaultSceneRoot) "None"))
      (EventDispatchers|AssignOnSystemFinished _returnvalue (delegate Custom|SystemFinished)))
    (:else
      (Utilities|FlowControl|Delay 0.2)
      (Actor|DestroyActor))))

(event Custom|PlayBlastSound
  (bind _returnvalue (Transformation|GetActorLocation))
  ;[1 1 1] Sound
  (bind _sound (Variables|Default|GetSound)
    (:then
      (Audio|PlaySoundatLocation _sound _returnvalue "0, 0, 0" 1.0 1.0 0.0 0 0 0 0)
      (Class|Actor|MakeNoise 1.0 (Game|Player|GetPlayerPawn 0) _returnvalue 0.0 "None"))
    (:else)))

(event EventBeginPlay
  (|CallParentFunction) ; This node is disabled and will not be called.\nDrag off pins to build functionality.
)

(event Collision|EventActorBeginOverlap
  (params (OtherActor :type Actor%20Object%20Reference)))

(event EventTick
  (params (DeltaSeconds :type Float%20%28single-precision%29)))

(event EventTrigger
  (|CallParentFunction)
  (EventDispatchers|BindEventtoOnActive (delegate Custom|SpawnBlastEffect)))

(fn ConstructionScript
  (|CallParentFunction))