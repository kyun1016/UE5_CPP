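; Attack component that carries out its owner's ranged attacks: a hitscan bullet and a targeted magic projectile.
; FireBullet line-traces for Pawns, while MagicSpell spawns a projectile toward a target and binds its impact event.
; Both paths send a damage message to the hit actor and report it to AI damage sensing.
; Only the projectile impact signals that the attack has ended.
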(event Custom|FireBullet
  (params (TraceStart :type Vector) (TraceEnd :type Vector) (DamageInfo :type S%20Damage%20Info%20Structure))
  (bind _outhit (Collision|LineTraceForObjects TraceStart TraceEnd (Utilities|Array|MakeArray "ObjectTypeQuery3") false 0 "None"))
  (if true
    (Class|BPIDamagable|TakeDamage(Message) (.HitActor (Collision|BreakHitResult _outhit)) DamageInfo)
    (Class|AISenseDamage|ReportDamageEvent (.HitActor (Collision|BreakHitResult _outhit)) (Components|GetOwner) (Utilities|Struct|BreakS_DamageInfo DamageInfo) (Transformation|GetActorLocation (Components|GetOwner)) "0, 0, 0" "None")))

(event Custom|OnProjectileHit
  (params (OtherActor :type Actor%20Object%20Reference) (Hit :type Hit%20Result%20Structure))
  (Class|BPIDamagable|TakeDamage(Message) OtherActor (stale Custom|MagicSpell DamageInfo))
  (Class|AISenseDamage|ReportDamageEvent OtherActor (Components|GetOwner) (Utilities|Struct|BreakS_DamageInfo (stale Custom|MagicSpell DamageInfo)) (Transformation|GetActorLocation (Components|GetOwner)) "0, 0, 0" "None")
  (Default|CallOnAttackEnded))

(event Custom|MagicSpell
  (params (SpawnTransform :type Transform) (Target :type Actor%20Object%20Reference) (DamageInfo :type S%20Damage%20Info%20Structure))
  (bind _returnvalue (Game|SpawnActorfromClass (Utilities|Array|Get(acopy) (Variables|Default|GetMagic)) SpawnTransform "Undefined" "MultiplyWithRoot" (Components|GetOwner) 1e+03 0.0 Target false 0))
  (EventDispatchers|BindEventtoOnProjectileImpact _returnvalue (delegate Custom|OnProjectileHit)))