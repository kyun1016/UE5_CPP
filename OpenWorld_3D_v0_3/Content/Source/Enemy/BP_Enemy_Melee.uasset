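; Melee sword enemy Blueprint that extends a parent enemy with attack, equip, unequip and block actions.
; Montage notifies time a forward sphere trace that damages pawns and spawn or destroy the hand-socketed sword.
; Blocking sets a flag on the damage component, whose OnBlocked event plays a reaction montage before ending the block.
; Attack, equip, unequip and block completions are reported through calls such as OnAttackEnd.
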(event OnBlocked(BPC_DamageSyatem)
  (params (CanBeParried :type Boolean))
  (Variables|Default|SetBlockingState "NewEnumerator2")
  (Animation|Montage|PlayMontage (Variables|Character|GetMesh) "/Game/Source/Enemy/Animation/Sword/Montage_Sword_Block_React.Montage_Sword_Block_React"
    (:OnCompleted
      _)
    (:OnInterrupted
      _))
  (CallFunction|EndBlock))

(event Custom|EndBlock
  (Variables|/Game/Source/DamageSystem/BPC_DamageSyatem.BPC_DamageSyatem_C|SetIsBlocking (Variables|Default|GetBPC_DamageSyatem) false)
  (Variables|Default|SetBlockingState "NewEnumerator0")
  (Default|CallOnBlockEnded))

(event Custom|StartBlock
  (Variables|/Game/Source/DamageSystem/BPC_DamageSyatem.BPC_DamageSyatem_C|SetIsBlocking (Variables|Default|GetBPC_DamageSyatem) true)
  (Variables|Default|SetBlockingState "NewEnumerator1")
  (Animation|Montage|PlayMontage (Variables|Character|GetMesh) "/Game/Source/Enemy/Animation/Sword/Montage_Sword_Block.Montage_Sword_Block"
    (:OnCompleted
      (if (Utilities|Enum|NotEqual(Enum) (Variables|Default|GetBlockingState) "NewEnumerator2")
        (CallFunction|EndBlock)))))

(event EventBeginPlay
  (|CallParentFunction))

(event EventAnimUnequipWeapon
  ;[1 1 1] Sheath Sword
  (bind _notifyname (Animation|Montage|PlayMontage (Variables|Character|GetMesh) "/Game/Source/Enemy/Animation/Sword/Montage_Sheath_Sword.Montage_Sheath_Sword")
    (:OnCompleted
      (Default|CallOnWeaponUnequipped))
    (:OnNotifyBegin
      (switch name _notifyname
        (:UnequipWeapon
          (Actor|DestroyActor (Variables|Default|GetWeaponActor))
          (Variables|Default|SetbIsWieldingWeapon false))))))

(event EventAnimEquipWeapon
  ;[1 1 1] Spawn Sword
  (bind _notifyname (Animation|Montage|PlayMontage (Variables|Character|GetMesh) "/Game/Source/Enemy/Animation/Sword/Montage_Withdraw_Sword.Montage_Withdraw_Sword")
    (:OnCompleted
      (Default|CallOnWeaponEquipped))
    (:OnNotifyBegin
      (switch name _notifyname
        (:EquipWeapon
          (bind _returnvalue (Game|SpawnActorfromClass "/Game/Source/Weapons/BP_Weapon_Sword.BP_Weapon_Sword_C" (Transformation|GetActorTransform) "Undefined" "MultiplyWithRoot" self 0))
          (bind _output_get (Variables|Default|SetWeaponActor _returnvalue))
          (Transformation|AttachComponentToComponent _output_get (Variables|Character|GetMesh) "hand_r_sword_socket" "SnapToTarget" "SnapToTarget" "SnapToTarget" true)
          (Variables|Default|SetbIsWieldingWeapon true))))))

(event EventAnimAttack
  (bind _returnvalue (Transformation|GetActorLocation))
  ;[1 1 1] Attack
  (Variables|Default|SetAttacking true)
  (bind _notifyname (Animation|Montage|PlayMontage (Variables|Character|GetMesh) "/Game/Source/Enemy/Animation/Sword/Montage_Slash_Sword.Montage_Slash_Sword")
    (:OnCompleted
      (Default|CallOnAttackEnd :!label _label)
      (Variables|Default|SetAttacking false))
    (:OnInterrupted
      (goto _label))
    (:OnNotifyBegin
      (switch name _notifyname
        (:Attack
          (bind (_outhit _returnvalue_2) (Collision|SphereTraceForObjects _returnvalue (+ _returnvalue (* "200.000000,200.000000,200.000000" (Transformation|GetActorForwardVector))) 2e+01 (Utilities|Array|MakeArray "ObjectTypeQuery3") false 0 "ForDuration"))
          (if _returnvalue_2
            (Class|BPIDamagable|TakeDamage(Message) (.HitActor (Collision|BreakHitResult _outhit)) (Variables|Default|GetDamage%20Info) self)))))))

(fn ConstructionScript
  (|CallParentFunction))