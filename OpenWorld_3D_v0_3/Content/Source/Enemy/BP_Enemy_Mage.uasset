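; Mage enemy character that fights at range with fireball spells and can teleport.
; The attack montage's notify fires a spell through BPCAttacks from the right hand toward the target.
; Teleport is a disguised high-speed AI flight: the mesh hides and ignores pawns while particle effects trail it, then walking is restored and the end dispatcher fires.
; Function overrides supply mage-specific movement speeds and attack/defend ranges.
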(event Custom|TeleportStart
  (params (Location :type Vector))
  (bind _charactermovement (Variables|Character|GetCharacterMovement))
  (bind _mesh (Variables|Character|GetMesh))
  ;[1 1 1] Teleport Start
  (if (not (Variables|Default|GetIsTeleporting))
    (Variables|Default|SetIsTeleporting true)
    (Pawn|Components|CharacterMovement|SetMovementMode _charactermovement "MOVE_Flying" 0)
    (Variables|/Script/Engine.CharacterMovementComponent|SetMaxFlySpeed _charactermovement 5e+03)
    (Variables|/Script/Engine.CharacterMovementComponent|SetMaxAcceleration _charactermovement 99999.0)
    (Rendering|SetVisibility _mesh false true)
    (Collision|SetCollisionResponsetoChannel _mesh "ECC_Pawn" "ECR_Ignore")
    (bind _returnvalue (Effects|SpawnEmitterAttached "/Game/Source/Projectiles/Particles/P_Gideon_Burden_DoT.P_Gideon_Burden_DoT" _mesh "Spine1"))
    (Variables|Default|SetTeleportBodyEffect _returnvalue)
    (bind _returnvalue_2 (Effects|SpawnEmitterAttached "/Game/Source/Projectiles/Particles/P_Gideon_Meteor_Trail.P_Gideon_Meteor_Trail" _mesh "Spine1"))
    (Variables|Default|SetTeleportTrailEffect _returnvalue_2)
    (Animation|StopAnimMontage 0)
    (AI|AIMoveTo self Location 0 15.0 false
      (:OnSuccess
        _)
      (:OnFail
        _))
    (CallFunction|TeleportEnd)
    (else
      (Utilities|FlowControl|DelayUntilNextTick)
      (Default|CallOnTeleportEnd))))

(event Custom|TeleportEnd
  (bind _charactermovement (Variables|Character|GetCharacterMovement))
  (bind _mesh (Variables|Character|GetMesh))
  ;[1 1 1] Teleport End
  (Components|Movement|StopMovementImmediately _charactermovement)
  (Pawn|Components|CharacterMovement|SetMovementMode _charactermovement "MOVE_Walking" 0)
  (Variables|/Script/Engine.CharacterMovementComponent|SetMaxAcceleration _charactermovement 2048.0)
  (Rendering|SetVisibility _mesh true true)
  (Collision|SetCollisionResponsetoChannel _mesh "ECC_Pawn" "ECR_Block")
  (Default|CallOnTeleportEnd)
  (Utilities|FlowControl|Delay 0.5)
  (Variables|Default|SetIsTeleporting false)
  (Utilities|FlowControl|Sequence
    (:then_0
      (bind _teleportbodyeffect (Variables|Default|GetTeleportBodyEffect)
        (:then
          (Components|DestroyComponent _teleportbodyeffect))
        (:else)))
    (:then_1
      (bind _teleporttraileffect (Variables|Default|GetTeleportTrailEffect)
        (:then
          (Components|DestroyComponent _teleporttraileffect))
        (:else)))))

(event EventBeginPlay
  (|CallParentFunction) ; This node is disabled and will not be called.\nDrag off pins to build functionality.
)

(event Collision|EventActorBeginOverlap
  (params (OtherActor :type Actor%20Object%20Reference)))

(event EventTick
  (params (DeltaSeconds :type Float%20%28single-precision%29)))

(event EventAnimAttack
  (params (AttackTarget :type Actor%20Object%20Reference))
  (bind _mesh (Variables|Character|GetMesh))
  (bind _returnvalue (Transformation|GetSocketLocation _mesh "RightHandMiddle1"))
  (bind _returnvalue_2 (+ _returnvalue "-5.000000,-5.000000,5.000000"))
  ;[1 1 1] Attack
  (bind _notifyname (Animation|Montage|PlayMontage (Variables|Character|GetMesh) "/Game/Source/Animation/Mixamo/Asset/Mage/Montage/Montage_Mage_Fireball.Montage_Mage_Fireball")
    (:OnCompleted
      (CallFunction|AttackEnd AttackTarget :!label _label))
    (:OnInterrupted
      (goto _label))
    (:OnNotifyBegin
      (switch name _notifyname
        (:Fire
          (Default|MagicSpell (Variables|Default|GetBPC_Attacks) (Math|Transform|MakeTransform _returnvalue_2 (Math|Rotator|FindLookatRotation _returnvalue_2 (Transformation|GetActorLocation AttackTarget)) "1.000000,1.000000,1.000000") AttackTarget (Variables|Default|GetDamageInfo)))))))

(fn ConstructionScript
  (|CallParentFunction))

(fn SetMovementSpeed
  (params (Speed :type E_MovementSpeed%20Enum :default "NewEnumerator0"))
  (return (Utilities|Select :Index Speed :NewEnumerator0 0.0 :NewEnumerator1 1.5e+02 :NewEnumerator2 2.5e+02 :NewEnumerator3 4e+02)))

(fn GetIdealRange
  (return 5e+02 7e+02))