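; Base enemy character that supplies health, damage, patrol route, combat range and movement speed tiers to its AI.
; BPCDamageSyatem handles damage, healing and death state, with a health bar widget created on BeginPlay and an explosion emitter on successful hits.
; Its delegates drive reactions through AIC_EnemyBase: hits halt movement and freeze the AI during a montage before it resumes attacking.
; Death enables ragdoll physics and stops the AI brain.
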(event Custom|HitResponse
  (params (DamageResponse :type E_DamageResponse%20Enum :default "NewEnumerator0"))
  (Components|Movement|StopMovementImmediately (Variables|Character|GetCharacterMovement))
  (Default|SetStateasFrozen (Variables|AI|GetAICEnemyBase))
  (Animation|Montage|PlayMontage (Variables|Character|GetMesh) (Variables|Default|GetHitReactionMontage)
    (:OnCompleted
      _)
    (:OnInterrupted
      _))
  (Default|SetStateasAttacking (Variables|AI|GetAICEnemyBase) 0 true))

(event Custom|Die
  (bind _mesh (Variables|Character|GetMesh))
  (bind _aicenemybase (Variables|AI|GetAICEnemyBase))
  (Physics|SetSimulatePhysics _mesh true)
  (Collision|SetCollisionEnabled _mesh "QueryAndPhysics")
  (AI|Logic|StopLogic (Variables|/Script/AIModule.AIController|GetBrainComponent _aicenemybase) "Dead")
  (Default|SetStateasDead _aicenemybase))

(event EventBeginPlay
  (bind _bpc_damagesyatem (Variables|Default|GetBPC_DamageSyatem))
  (bind _returnvalue (UserInterface|CreateWidget "/Game/Source/DamageSystem/W_HealthBar.W_HealthBar_C" 0 self))
  (UserInterface|SetWidget (Variables|Default|GetHealthBar) _returnvalue)
  (EventDispatchers|BindEventtoOnDeath _bpc_damagesyatem (EventDispatchers|CreateEvent :!event Custom|Die))
  (EventDispatchers|BindEventtoOnDeamageResponse _bpc_damagesyatem (EventDispatchers|CreateEvent :!event Custom|HitResponse))
  (bind _asaic_enemy_base (Utilities|Casting|CastToAIC_EnemyBase (AI|GetAIController self)))
  (Variables|AI|SetAICEnemyBase _asaic_enemy_base))

(fn ConstructionScript)

(fn GetCurrentHealth
  (return (Variables|/Game/Source/DamageSystem/BPC_DamageSyatem.BPC_DamageSyatem_C|GetHealth (Variables|Default|GetBPC_DamageSyatem))))

(fn GetIdealRange
  (return 1.5e+02 3.5e+02))

(fn GetMaxHealth
  (return (Variables|/Game/Source/DamageSystem/BPC_DamageSyatem.BPC_DamageSyatem_C|GetMaxHealth (Variables|Default|GetBPC_DamageSyatem))))

(fn GetPatrolRoute
  (return (Variables|AI|GetPatrolRoute)))

(fn Heal
  (params (Amount :type Float%20%28double-precision%29))
  (bind _health (Default|Heal (Variables|Default|GetBPC_DamageSyatem) Amount))
  (return _health))

(fn IsDead
  (return (Variables|/Game/Source/DamageSystem/BPC_DamageSyatem.BPC_DamageSyatem_C|GetIsDead (Variables|Default|GetBPC_DamageSyatem))))

(fn SetMovementSpeed
  (params (Speed :type E_MovementSpeed%20Enum :default "NewEnumerator0"))
  (bind _output_get (Variables|/Script/Engine.CharacterMovementComponent|SetMaxWalkSpeed (Variables|Character|GetCharacterMovement) (Utilities|Select :Index Speed :NewEnumerator0 0.0 :NewEnumerator1 1e+02 :NewEnumerator2 3e+02 :NewEnumerator3 5e+02)))
  (return _output_get))

(fn TakeDamage
  (params (DamageInfo :type S%20Damage%20Info%20Structure))
  (bind _wasdamaged (Default|TakeDamage (Variables|Default|GetBPC_DamageSyatem) DamageInfo))
  (if _wasdamaged
    (Effects|SpawnEmitteratLocation "/Game/Source/Particles/P_Explosion.P_Explosion" (Transformation|GetActorLocation))
    (return _wasdamaged)))