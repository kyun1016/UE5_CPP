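; BP_Enemy_Ranged is an enemy character that equips a rifle on BeginPlay and can chase and attack the player.
; Equipping uses a montage notify to spawn and socket the rifle, then broadcasts equip events.
; ChasePlayer loops AIMoveTo with a delay, triggering Attack on arrival, but nothing here starts it.
; Attack and unequip still use sword montages, and unequip destroys SwordActor rather than the spawned WeaponActor.
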(event Custom|Attack
  ;[1 1 1] Attack
  (Animation|Montage|PlayMontage (Variables|Character|GetMesh) "/Game/Character/Enemy/Animation/Montage_Sword_And_Shield_Slash.Montage_Sword_And_Shield_Slash"
    (:OnCompleted
      _)
    (:OnInterrupted
      _))
  (Default|CallOnAttackEnd))

(event Custom|ChasePlayer
  ;[1 1 1] Chase Player
  (AI|AIMoveTo self "0, 0, 0" (Game|GetPlayerCharacter 0) 1.5e+02 false
    (:OnSuccess
      (CallFunction|Attack)
      (Utilities|FlowControl|Delay 2.0)
      (CallFunction|ChasePlayer))
    (:OnFail
      (Utilities|FlowControl|Delay 2.0)
      (CallFunction|ChasePlayer))))

(event EventUnequipWeapon
  ;[1 1 1] Sheath Sword
  (bind _notifyname (Animation|Montage|PlayMontage (Variables|Character|GetMesh) "/Game/Character/Enemy/Animation/Montage_Sheath_Sword.Montage_Sheath_Sword")
    (:OnCompleted
      (Default|CallOnSheathSword))
    (:OnNotifyBegin
      (switch name _notifyname
        (:DropSword
          (Actor|DestroyActor (Variables|Default|GetSwordActor))
          (Variables|Default|SetIsWieldingWeapon false))))))

(event EventBeginPlay
  ;[1 1 1] Begin Play
  (CallFunction|EquipWeapon))

(event EventEquipWeapon
  ;[1 1 1] Spawn Sword
  (bind _notifyname (Animation|Montage|PlayMontage (Variables|Character|GetMesh) "/Game/Character/Enemy/Animation/Montage_Withdrawing_Sword.Montage_Withdrawing_Sword")
    (:OnCompleted
      (Default|CallOnWieldSword))
    (:OnNotifyBegin
      (switch name _notifyname
        (:HoldSword
          (bind _returnvalue (Game|SpawnActorfromClass "/Game/Character/Weapons/BP_Weapon_Rifle.BP_Weapon_Rifle_C" (Transformation|GetActorTransform) "Undefined" "MultiplyWithRoot" 0 0))
          (bind _output_get (Variables|Default|SetWeaponActor _returnvalue))
          (Transformation|AttachComponentToComponent _output_get (Variables|Character|GetMesh) "hand_r_rifle_socket" "SnapToTarget" "SnapToTarget" "SnapToTarget" true)
          (Variables|Default|SetIsWieldingWeapon true)
          (Default|CallOnWeaponEquipped))))))

(fn ConstructionScript)