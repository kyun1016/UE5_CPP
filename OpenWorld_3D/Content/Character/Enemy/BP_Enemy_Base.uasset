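; Base enemy character that fights with a sword and exposes combat ranges, a patrol route and enum-driven walk speeds.
; Attack, equip and unequip play montages and fire completion dispatchers for callers.
; Montage notifies time spawning the sword onto the hand socket and destroying it when sheathed.
; ChasePlayer is a self-repeating move-to-player loop that attacks on arrival, though nothing in this graph starts it.
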(event Custom|Attack
  ;[1 1 1] Attack
  (Animation|Montage|PlayMontage (Variables|Character|GetMesh) "/Game/Character/Enemy/Animation/Montage_Sword_And_Shield_Slash.Montage_Sword_And_Shield_Slash"
    (:OnCompleted
      _)
    (:OnInterrupted
      _))
  (Default|CallOnAttackEnd))

(event Custom|ChasePlayer
  ;[1 1 1] Chase Player
  (AI|AIMoveTo self "0, 0, 0" (Game|GetPlayerCharacter 0) 1.5e+02 false
    (:OnSuccess
      (CallFunction|Attack)
      (Utilities|FlowControl|Delay 2.0)
      (CallFunction|ChasePlayer))
    (:OnFail
      (Utilities|FlowControl|Delay 2.0)
      (CallFunction|ChasePlayer))))

(event EventUnequipWeapon
  ;[1 1 1] Sheath Sword
  (bind _notifyname (Animation|Montage|PlayMontage (Variables|Character|GetMesh) "/Game/Character/Enemy/Animation/Montage_Sheath_Sword.Montage_Sheath_Sword")
    (:OnCompleted
      (Default|CallOnWeaponUnequipped))
    (:OnNotifyBegin
      (switch name _notifyname
        (:DropSword
          (Actor|DestroyActor (Variables|Default|GetWeaponActor))
          (Variables|Default|SetIsWieldingWeapon false))))))

(event EventBeginPlay
  ;[1 1 1] Begin Play
)

(event EventEquipWeapon
  ;[1 1 1] Spawn Sword
  (bind _notifyname (Animation|Montage|PlayMontage (Variables|Character|GetMesh) "/Game/Character/Enemy/Animation/Montage_Withdrawing_Sword.Montage_Withdrawing_Sword")
    (:OnCompleted
      (Default|CallOnWeaponEquipped))
    (:OnNotifyBegin
      (switch name _notifyname
        (:HoldSword
          (bind _returnvalue (Game|SpawnActorfromClass "/Game/Character/Weapons/BP_Weapon_Sword.BP_Weapon_Sword_C" (Transformation|GetActorTransform) "Undefined" "MultiplyWithRoot" 0 0))
          (bind _output_get (Variables|Default|SetWeaponActor _returnvalue))
          (Transformation|AttachComponentToComponent _output_get (Variables|Character|GetMesh) "hand_r_sword_socket" "SnapToTarget" "SnapToTarget" "SnapToTarget" true)
          (Variables|Default|SetIsWieldingWeapon true))))))

(fn ConstructionScript)

(fn GetIdealRange
  (return 1.5e+02 3.5e+02))

(fn GetPatrolRoute
  (return (Variables|AI|GetPatrolRoute)))

(fn SetMovementSpeed
  (params (Speed :type E_MovementSpeed%20Enum :default "NewEnumerator0"))
  (bind _output_get (Variables|/Script/Engine.CharacterMovementComponent|SetMaxWalkSpeed (Variables|Character|GetCharacterMovement) (Utilities|Select :Index Speed :NewEnumerator0 0.0 :NewEnumerator1 1e+02 :NewEnumerator2 3e+02 :NewEnumerator3 5e+02)))
  (return _output_get))